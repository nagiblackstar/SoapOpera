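; Silverfish enemy that chases the player while they are inside its CharacterRegister detection volume.
; On Tick it moves straight toward the cached ThirdPersonCharacter and yaws its capsule to face them, holding still within a short horizontal distance.
; Attackbox overlaps only toggle an Attacking flag, which nothing in these graphs reads.
; Hurtbox sends DeathMessage to any actor that overlaps it, without checking for the player.
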(event OnComponentEndOverlap(CharacterRegister)
  (params (OverlappedComponent :type Primitive%20Component%20Object%20Reference) (OtherActor :type Actor%20Object%20Reference) (OtherComp :type Primitive%20Component%20Object%20Reference) (OtherBodyIndex :type Integer))
  (if (== OtherActor (Variables|Default|GetPlayer))
    (Variables|Default|SetChasing false)))

(event OnComponentBeginOverlap(Hurtbox)
  (params (OverlappedComponent :type Primitive%20Component%20Object%20Reference) (OtherActor :type Actor%20Object%20Reference) (OtherComp :type Primitive%20Component%20Object%20Reference) (OtherBodyIndex :type Integer) (bFromSweep :type Boolean) (SweepResult :type Hit%20Result%20Structure%20%28by%20ref%29))
  (Class|CharacterBPI|Death(Message) OtherActor))

(event OnComponentBeginOverlap(CharacterRegister)
  (params (OverlappedComponent :type Primitive%20Component%20Object%20Reference) (OtherActor :type Actor%20Object%20Reference) (OtherComp :type Primitive%20Component%20Object%20Reference) (OtherBodyIndex :type Integer) (bFromSweep :type Boolean) (SweepResult :type Hit%20Result%20Structure%20%28by%20ref%29))
  (if (== OtherActor (Variables|Default|GetPlayer))
    (Variables|Default|SetChasing true)))

(event OnComponentBeginOverlap(Attackbox)
  (params (OverlappedComponent :type Primitive%20Component%20Object%20Reference) (OtherActor :type Actor%20Object%20Reference) (OtherComp :type Primitive%20Component%20Object%20Reference) (OtherBodyIndex :type Integer) (bFromSweep :type Boolean) (SweepResult :type Hit%20Result%20Structure%20%28by%20ref%29))
  (if (== OtherActor (Variables|Default|GetPlayer))
    (Variables|Default|SetAttacking true)))

(event OnComponentEndOverlap(Attackbox)
  (params (OverlappedComponent :type Primitive%20Component%20Object%20Reference) (OtherActor :type Actor%20Object%20Reference) (OtherComp :type Primitive%20Component%20Object%20Reference) (OtherBodyIndex :type Integer))
  (if (== OtherActor (Variables|Default|GetPlayer))
    (Variables|Default|SetAttacking false)))

(event EventBeginPlay
  (bind _asthird_person_character (Utilities|Casting|CastToThirdPersonCharacter (Game|Player|GetPlayerPawn 0)))
  (Variables|Default|SetPlayer _asthird_person_character))

(event EventTick
  (params (DeltaSeconds :type Float%20%28single-precision%29))
  (bind _self self)
  (bind _player (Variables|Default|GetPlayer))
  (bind _returnvalue (Transformation|GetActorLocation _self))
  (bind _returnvalue_2 (Transformation|GetActorLocation _player))
  (bind _returnvalue_3 (- _returnvalue_2 _returnvalue))
  (if (Variables|Default|GetChasing)
    (Math|Float|CompareFloat (Math|Vector|VectorLengthXY _returnvalue_3) 2e+02
      (:>
        (Pawn|Input|AddMovementInput (Math|Vector|Normalize _returnvalue_3) (Variables|Default|GetSpeed) false)
        (Transformation|SetWorldRotation (Variables|Collision|GetCapsuleComponent) (Math|Rotator|MakeRotator 0.0 0.0 (.Yaw (Math|Rotator|BreakRotator (Math|Rotator|FindLookatRotation (Transformation|GetActorLocation self) (Transformation|GetActorLocation (Variables|Default|GetPlayer)))))) false false)))))

(fn ConstructionScript)