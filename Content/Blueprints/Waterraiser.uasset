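; Waterraiser is a trigger actor that moves the level's Waterscape actor vertically to the height of its End component when the player enters it.
; On BeginPlay it caches the Waterscape, and a Heightcheck overlap by the player pawn records that actor's location and starts a timeline.
; The timeline lerps only Z, with play rate set from the height difference divided by a constant, and the trigger destroys itself on finish.
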(event OnComponentBeginOverlap(Heightcheck)
  (params (OverlappedComponent :type Primitive%20Component%20Object%20Reference) (OtherActor :type Actor%20Object%20Reference) (OtherComp :type Primitive%20Component%20Object%20Reference) (OtherBodyIndex :type Integer) (bFromSweep :type Boolean) (SweepResult :type Hit%20Result%20Structure%20%28by%20ref%29))
  (if (== OtherActor (Game|Player|GetPlayerPawn 0))
    (Variables|Default|SetWaterscape_Loc (Transformation|GetActorLocation (Variables|Default|GetWaterscape)))
    (bind _output_get (Variables|Default|SetWaterspeed (/ (- (.Z (Math|Vector|BreakVector (Transformation|GetWorldLocation (Variables|Default|GetEnd)))) (.Z (Math|Vector|BreakVector (Transformation|GetActorLocation (Variables|Default|GetWaterscape))))) 7e+02)))
    (Components|Timeline|SetPlayRate (Variables|Default|GetWater%20Timeline) _output_get)
    (bind _leggo (Timeline|Water%20Timeline Play)
      (:Update
        (Transformation|SetActorLocation (Variables|Default|GetWaterscape) (Math|Vector|Lerp(Vector) (Variables|Default|GetWaterscape_Loc) (Math|Vector|MakeVector (.X (Math|Vector|BreakVector (Variables|Default|GetWaterscape_Loc))) (.Y (Math|Vector|BreakVector (Variables|Default|GetWaterscape_Loc))) (.Z (Math|Vector|BreakVector (Transformation|GetWorldLocation (Variables|Default|GetEnd))))) _leggo) false false))
      (:Finished
        (Actor|DestroyActor)))))

(event EventBeginPlay
  (bind _returnvalue (Actor|GetActorOfClass "/Game/Blueprints/Waterscape.Waterscape_C"))
  (Variables|Default|SetWaterscape _returnvalue))

(event Collision|EventActorBeginOverlap
  (params (OtherActor :type Actor%20Object%20Reference)))

(event EventTick
  (params (DeltaSeconds :type Float%20%28single-precision%29)))

(fn ConstructionScript)