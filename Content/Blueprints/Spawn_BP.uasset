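; Spawn_BP is a one-shot trigger that spawns a Silverfish_BP enemy when the player enters its SpawnCheck volume.
; On overlap it confirms the actor is the player pawn, then spawns the silverfish at the volume's location and rotation and gives it a default controller.
; A HasSpawned flag, reset at BeginPlay, prevents any further spawns.
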(event OnComponentBeginOverlap(SpawnCheck)
  (params (OverlappedComponent :type Primitive%20Component%20Object%20Reference) (OtherActor :type Actor%20Object%20Reference) (OtherComp :type Primitive%20Component%20Object%20Reference) (OtherBodyIndex :type Integer) (bFromSweep :type Boolean) (SweepResult :type Hit%20Result%20Structure%20%28by%20ref%29))
  (bind _spawncheck (Variables|Default|GetSpawnCheck))
  (bind _returnvalue (Transformation|GetWorldTransform _spawncheck))
  (if (== OtherActor (Game|Player|GetPlayerPawn 0))
    (if (not (Variables|Default|GetHasSpawned))
      (bind _returnvalue_2 (Game|SpawnActorfromClass "/Game/Enemy/Enemy_Blueprint/Silverfish_BP.Silverfish_BP_C" (Math|Transform|MakeTransform (.location _returnvalue) (.rotation _returnvalue) "1,1,1") "Undefined" 0 0))
      (Pawn|SpawnDefaultController _returnvalue_2)
      (Variables|Default|SetHasSpawned true))))

(event EventBeginPlay
  (Variables|Default|SetHasSpawned false))

(fn ConstructionScript)