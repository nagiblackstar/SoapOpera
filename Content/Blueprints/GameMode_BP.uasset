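; Game mode that manages saving and restoring the player's position through a single save slot using SaveGame_BP.
; BeginPlay creates the save if missing, otherwise moves the ThirdPersonCharacter to the saved transform when UseSaveLocation is set.
; SaveGame stores that transform and sets the flag; LoadGame reopens the current level, while RestartLevel deletes the save and restarts.
; ChangeLevels clears the flag, but loads from an empty slot name rather than "save1".
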(event Custom|SaveGame
  (bind _returnvalue (SaveGame|LoadGamefromSlot "save1"))
  (bind _assave_game_bp (Utilities|Casting|CastToSaveGame_BP _returnvalue)
    (:then
      (bind _output_get (Variables|/Game/Blueprints/SaveGame_BP.SaveGame_BP_C|SetPlayerLocation _assave_game_bp (Transformation|GetActorTransform (.AsThird%20Person%20Character (Utilities|Casting|CastToThirdPersonCharacter (Game|GetPlayerCharacter 0))))))
      (Development|PrintString (Utilities|String|ToString(Transform) _output_get))
      (Variables|/Game/Blueprints/SaveGame_BP.SaveGame_BP_C|SetUseSaveLocation _assave_game_bp true)
      (SaveGame|SaveGametoSlot _assave_game_bp "save1"))
    (:CastFailed
      (Development|PrintString "cast failed :("))))

(event Custom|LoadGame
  (bind _returnvalue (Game|GetCurrentLevelName true))
  (Game|OpenLevel(byName) (Utilities|String|StringToName _returnvalue)))

(event Custom|RestartLevel
  (SaveGame|DeleteGameinSlot "save1")
  (Development|ExecuteConsoleCommand "RestartLevel" 0))

(event Custom|ChangeLevels
  (bind _returnvalue (SaveGame|LoadGamefromSlot))
  (bind _assave_game_bp (Utilities|Casting|CastToSaveGame_BP _returnvalue))
  (Variables|/Game/Blueprints/SaveGame_BP.SaveGame_BP_C|SetUseSaveLocation _assave_game_bp false)
  (SaveGame|SaveGametoSlot _assave_game_bp "save1"))

(event EventBeginPlay
  (Development|PrintString "BeginPlay")
  (bind _returnvalue (SaveGame|DoesSaveGameExist "save1"))
  (if _returnvalue
    (bind _returnvalue_2 (SaveGame|LoadGamefromSlot "save1"))
    (bind _assave_game_bp (Utilities|Casting|CastToSaveGame_BP _returnvalue_2))
    (if (Variables|/Game/Blueprints/SaveGame_BP.SaveGame_BP_C|GetUseSaveLocation _assave_game_bp)
      (bind _asthird_person_character (Utilities|Casting|CastToThirdPersonCharacter (Game|GetPlayerCharacter 0)))
      (Transformation|SetActorTransform _asthird_person_character (Variables|/Game/Blueprints/SaveGame_BP.SaveGame_BP_C|GetPlayerLocation _assave_game_bp)))
    (else
      (bind _returnvalue_3 (SaveGame|CreateSaveGameObject "/Game/Blueprints/SaveGame_BP.SaveGame_BP_C"))
      (SaveGame|SaveGametoSlot _returnvalue_3 "save1"))))

(event EventTick
  (params (DeltaSeconds :type Float%20%28single-precision%29)))

(fn ConstructionScript)