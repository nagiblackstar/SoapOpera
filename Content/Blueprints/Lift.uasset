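; Lift actor that moves its Cube from a Start point to an End point when another actor overlaps its Box trigger.
; A timeline drives the lerp between the two world locations, with its play rate set from LiftSpeed on BeginPlay.
; End overlap does nothing, so the lift has no return logic.
; BeginPlay also caches a Waterscape actor, but the node that would move it relative to End is unconnected.
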(event OnComponentBeginOverlap(Box)
  (params (OverlappedComponent :type Primitive%20Component%20Object%20Reference) (OtherActor :type Actor%20Object%20Reference) (OtherComp :type Primitive%20Component%20Object%20Reference) (OtherBodyIndex :type Integer) (bFromSweep :type Boolean) (SweepResult :type Hit%20Result%20Structure%20%28by%20ref%29))
  (if (not (== OtherActor self))
    (bind _speed (Timeline|Lift_Timeline Play)
      (:Update
        (Transformation|SetWorldLocation (Variables|Default|GetCube) (Math|Vector|Lerp(Vector) (Transformation|GetWorldLocation (Variables|Default|GetStart)) (Transformation|GetWorldLocation (Variables|Default|GetEnd)) _speed) false false)))))

(event OnComponentEndOverlap(Box)
  (params (OverlappedComponent :type Primitive%20Component%20Object%20Reference) (OtherActor :type Actor%20Object%20Reference) (OtherComp :type Primitive%20Component%20Object%20Reference) (OtherBodyIndex :type Integer))
  (if (== OtherActor self)
    _))

(event EventBeginPlay
  (Components|Timeline|SetPlayRate (Variables|Default|GetLift_Timeline) (Variables|Default|GetLift_Speed))
  (bind _returnvalue (Actor|GetActorOfClass "/Game/Blueprints/Waterscape.Waterscape_C"))
  (Variables|Default|SetWaterscape _returnvalue))

(fn ConstructionScript)