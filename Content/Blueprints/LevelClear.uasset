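; LevelClear is a trigger actor that ends the level when the player pawn enters its box.
; On the first overlap it switches the ThirdPersonCharacter from its follow camera to its level-clear camera and disables input.
; It briefly shows a LevelClearMessage widget, then deletes the save slot and opens the main menu level.
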(event OnComponentBeginOverlap(Box)
  (params (OverlappedComponent :type Primitive%20Component%20Object%20Reference) (OtherActor :type Actor%20Object%20Reference) (OtherComp :type Primitive%20Component%20Object%20Reference) (OtherBodyIndex :type Integer) (bFromSweep :type Boolean) (SweepResult :type Hit%20Result%20Structure%20%28by%20ref%29))
  (bind _returnvalue (Game|Player|GetPlayerPawn 0))
  (if (== OtherActor _returnvalue)
    (Utilities|FlowControl|DoOnce false
      (:Completed
        (bind _asthird_person_character (Utilities|Casting|CastToThirdPersonCharacter _returnvalue))
        (Components|Activation|SetActive (Variables|/Game/ThirdPersonBP/Blueprints/ThirdPersonCharacter.ThirdPersonCharacter_C|GetFollowCamera _asthird_person_character) false false)
        (Components|Activation|SetActive (Variables|/Game/ThirdPersonBP/Blueprints/ThirdPersonCharacter.ThirdPersonCharacter_C|GetLevelClearCam _asthird_person_character) true false)
        (Input|DisableInput _asthird_person_character 0)
        (bind _returnvalue_2 (UserInterface|CreateWidget "/Game/Blueprints/LevelClearMessage.LevelClearMessage_C" (Game|GetPlayerController 0)))
        (bind _output_get (Variables|Default|SetLevelClearMessage _returnvalue_2))
        (UserInterface|Viewport|AddtoViewport _output_get 0)
        (Utilities|FlowControl|Delay 2.0)
        (Widget|RemovefromParent (Variables|Default|GetLevelClearMessage))
        (SaveGame|DeleteGameinSlot "save1")
        (Game|OpenLevel(byName) "MainMenuLevel")))))

(event EventBeginPlay)

(event Collision|EventActorBeginOverlap
  (params (OtherActor :type Actor%20Object%20Reference)))

(event EventTick
  (params (DeltaSeconds :type Float%20%28single-precision%29)))

(fn ConstructionScript)