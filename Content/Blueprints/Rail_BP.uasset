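; Rail actor that carries the player along a rail when their pawn enters the Launchbox trigger.
; On overlap it snaps the pawn to the spline's first point, facing the second, then plays Rail_Timeline from the start.
; The timeline's Speed track lerps the pawn's location between those two points, so travel is a straight line that ignores spline curvature and any further points.
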(event OnComponentBeginOverlap(Launchbox)
  (params (OverlappedComponent :type Primitive%20Component%20Object%20Reference) (OtherActor :type Actor%20Object%20Reference) (OtherComp :type Primitive%20Component%20Object%20Reference) (OtherBodyIndex :type Integer) (bFromSweep :type Boolean) (SweepResult :type Hit%20Result%20Structure%20%28by%20ref%29))
  (bind _returnvalue (Game|Player|GetPlayerPawn 0))
  (bind _spline (Variables|Default|GetSpline))
  (bind _spline_2 (Variables|Default|GetSpline))
  (bind _returnvalue_2 (Class|SplineComponent|GetLocationatSplineInputKey _spline 1.0 "World"))
  (bind _returnvalue_3 (Class|SplineComponent|GetLocationatSplineInputKey _spline_2 0.0 "World"))
  (if (== OtherActor (Game|Player|GetPlayerPawn 0))
    (Transformation|SetActorLocationAndRotation _returnvalue _returnvalue_3 (Math|Conversions|RotationFromXVector (Math|Vector|Normalize (- _returnvalue_2 _returnvalue_3))))
    (bind _speed (Timeline|Rail_Timeline PlayFromStart)
      (:Update
        (Transformation|SetActorLocation _returnvalue (Math|Vector|Lerp(Vector) _returnvalue_3 _returnvalue_2 _speed) false false)))))

(event EventBeginPlay
  (bind _asthird_person_character (Utilities|Casting|CastToThirdPersonCharacter (Game|Player|GetPlayerPawn 0)))
  (Variables|Default|SetPlayer _asthird_person_character))

(fn ConstructionScript)